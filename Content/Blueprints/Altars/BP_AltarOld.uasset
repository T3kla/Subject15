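; BP_AltarOld is an altar actor built from a roof cone, hexagon base, cylinder base, light column and particle system, with no runtime logic.
; Its Construction Script applies the particle template and per-part materials from variables.
; It also sets the roof cone's relative height and the light column's vertical scale from variables, so each altar variant is configurable in the editor.
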(event EventBeginPlay)

(event Collision|EventActorBeginOverlap
  (params (OtherActor :type Actor%20Object%20Reference)))

(event EventTick
  (params (DeltaSeconds :type Float%20%28single-precision%29)))

(fn ConstructionScript
  (Effects|Components|ParticleSystem|SetTemplate (Variables|Default|GetParticleSystem) (Variables|Default|GetTemplate))
  (Rendering|Material|SetMaterial (Variables|Default|GetRoofCone) 0 (Variables|Default|GetConeMaterial))
  (Rendering|Material|SetMaterial (Variables|Default|GetBaseHexagon) 0 (Variables|Default|GetBaseHexagonMaterial))
  (Rendering|Material|SetMaterial (Variables|Default|GetBaseCylinder) 0 (Variables|Default|GetBaseCylinderMaterial))
  (Rendering|Material|SetMaterial (Variables|Default|GetLightColumn) 0 (Variables|Default|GetLightColumnMaterial))
  (Transformation|SetRelativeLocation (Variables|Default|GetRoofCone) (Math|Vector|MakeVector 0.0 0.0 (Variables|Default|GetZPositionRoofCone)) false false)
  (Transformation|SetRelativeScale3D (Variables|Default|GetLightColumn) (Math|Vector|MakeVector 1.0 1.0 (Variables|Default|GetZScaleLightCol))))