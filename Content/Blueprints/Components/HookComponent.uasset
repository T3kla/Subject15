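; Actor component that gives its owning Character a grappling hook, triggered by ExecHookEvent with a camera and laser beam component.
; It line traces from the owner along the camera's forward vector, leaving persistent debug lines.
; On a hit it shows the beam from camera to impact, launches the character upward, then toward that point after a short delay.
; A delayed reset hides the beam and re-enables the hook, also after a miss.
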(event Custom|ExecHookEvent
  (params (PlayerCam :type Camera%20Component%20Object%20Reference) (LaserComponent :type Particle%20System%20Component%20Object%20Reference))
  (bind _returnvalue (Components|GetOwner))
  (bind _returnvalue_2 (Transformation|GetActorLocation _returnvalue))
  (Variables|Default|SetLaser LaserComponent)
  (Variables|Default|SetCameraPlayer PlayerCam)
  (if (Variables|Default|GetCanGrappleHook)
    (Variables|Default|SetCanGrappleHook false)
    (bind (_outhit _returnvalue_3) (Collision|LineTraceByChannel _returnvalue_2 (+ _returnvalue_2 (* (Math|Vector|GetForwardVector PlayerCam) 2e+03)) "TraceTypeQuery1" false 0 "Persistent"))
    (if _returnvalue_3
      (Variables|Default|SetHookLocation (.Location (Collision|BreakHitResult _outhit)))
      (CallFunction|ShootHook (Variables|Default|GetCameraPlayer))
      (bind _ascharacter (Utilities|Casting|CastToCharacter (Components|GetOwner)))
      (Character|LaunchCharacter _ascharacter "0, 0,500.000000" true true)
      (Utilities|FlowControl|Delay 0.2)
      (Character|LaunchCharacter _ascharacter (* (- (Variables|Default|GetHookLocation) (Transformation|GetActorLocation (Components|GetOwner))) 1.5) false false)
      (Utilities|FlowControl|Delay 0.5)
      (CallFunction|ResetGrappleHook)
      (else
        (Utilities|FlowControl|Delay 0.5)
        (CallFunction|ResetGrappleHook)))))

(fn ResetGrappleHook
  (Variables|Default|SetTimerHandle 0.0)
  (Rendering|SetVisibility (Variables|Default|GetLaser) false false)
  (Variables|Default|SetCanGrappleHook true))

(fn ShootHook
  (params (Camera :type Camera%20Component%20Object%20Reference))
  (Rendering|SetVisibility (Variables|Default|GetLaser) true false)
  (Class|ParticleSystemComponent|SetBeamSourcePoint (Variables|Default|GetLaser) 0 (Transformation|GetWorldLocation Camera))
  (Class|ParticleSystemComponent|SetBeamTargetPoint (Variables|Default|GetLaser) 0 (Variables|Default|GetHookLocation)))