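; BP_TriggerKill is a kill trigger that restarts the current level when an actor tagged Player overlaps it.
; The overlap sets IsInside, which Tick polls to disable player input, show a ResetLevel widget, wait for Duration and reopen the level by name.
; Tick clears Paused just before checking it, so the widget is created again every frame while IsInside stays true.
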(event Collision|EventActorBeginOverlap
  (params (OtherActor :type Actor%20Object%20Reference))
  (if (Actor|ActorHasTag OtherActor "Player")
    (Variables|Default|SetIsInside true)))

(event EventTick
  (params (DeltaSeconds :type Float%20%28single-precision%29))
  (if (Variables|Default|GetIsInside)
    (Input|DisableInput (Game|GetPlayerCharacter 0) (Game|GetPlayerController 0))
    (Variables|Default|SetPaused false)
    (if (not (Variables|Default|GetPaused))
      (bind _returnvalue (UserInterface|CreateWidget "/Game/Blueprints/ResetLevel.ResetLevel_C"))
      (UserInterface|Viewport|AddtoViewport _returnvalue 4)
      (Utilities|FlowControl|Delay (Variables|Default|GetDuration))
      (bind _returnvalue_2 (Game|GetCurrentLevelName true))
      (Game|OpenLevel(byName) (Utilities|String|StringToName _returnvalue_2)))))

(fn ConstructionScript)