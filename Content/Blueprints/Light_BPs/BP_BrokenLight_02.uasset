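; BP_BrokenLight_02 is a broken light actor whose rect light blinks on and off continuously during play.
; From BeginPlay, a FlipFlop sets the RectLight's visibility, then a 0.3-second Delay loops back into it, giving an evenly timed blink rather than a random flicker.
; The construction script applies radius and intensity variables to the RectLight's attenuation radius and intensity.
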(event EventBeginPlay
  (bind _isa (Utilities|FlowControl|FlipFlop :!label _label)
    (:A
      _)
    (:B
      _))
  (Rendering|SetVisibility (Variables|Default|GetRectLight) _isa false)
  (Utilities|FlowControl|Delay 0.3)
  (goto _label))

(fn ConstructionScript
  (Rendering|Lighting|SetAttenuationRadius (Variables|Default|GetRectLight) (Variables|Default|GetNew%20Radius))
  (Rendering|Components|Light|SetIntensity (Variables|Default|GetRectLight) (Variables|Default|GetNew%20Intensity)))