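; BP_Light_08 is a light fixture actor pairing the Light08 component with a configurable Light component.
; The construction script applies LightMaterial to material slot 1 of Light08 and sets the light's intensity, attenuation radius and color from variables.
; The event graph holds only empty default events, so the Blueprint adds no runtime logic.
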(event EventBeginPlay)

(event Collision|EventActorBeginOverlap
  (params (OtherActor :type Actor%20Object%20Reference)))

(event EventTick
  (params (DeltaSeconds :type Float%20%28single-precision%29)))

(fn ConstructionScript
  (Rendering|Material|SetMaterial (Variables|Default|GetLight_08) 1 (Variables|Default|GetLightMaterial))
  (Rendering|Components|Light|SetIntensity (Variables|Default|GetLight) (Variables|Default|GetNew%20Intensity))
  (Rendering|Lighting|SetAttenuationRadius (Variables|Default|GetLight) (Variables|Default|GetNew%20Radius))
  (Rendering|Components|Light|SetLightColor (Variables|Default|GetLight) (Variables|Default|GetNew%20Light%20Color) true))