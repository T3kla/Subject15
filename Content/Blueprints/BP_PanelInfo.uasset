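; BP_PanelInfo is an info panel actor that displays a title, description and version as text render components.
; Its construction script copies the three text variables into their components and applies one shared color variable to all of them.
; The event graph holds only disabled placeholder events, so the panel has no runtime logic.
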(event EventBeginPlay)

(event Collision|EventActorBeginOverlap
  (params (OtherActor :type Actor%20Object%20Reference)))

(event EventTick
  (params (DeltaSeconds :type Float%20%28single-precision%29)))

(fn ConstructionScript
  (Rendering|Components|TextRender|SetText (Variables|Default|GetTitle) (Variables|Default|GetTitleText))
  (Rendering|Components|TextRender|SetText (Variables|Default|GetDescription) (Variables|Default|GetDescriptionText))
  (Rendering|Components|TextRender|SetText (Variables|Default|GetVersion) (Variables|Default|GetVersionText))
  (Rendering|Components|TextRender|SetTextRenderColor (Variables|Default|GetDescription) (Variables|Default|GetColor))
  (Rendering|Components|TextRender|SetTextRenderColor (Variables|Default|GetTitle) (Variables|Default|GetColor))
  (Rendering|Components|TextRender|SetTextRenderColor (Variables|Default|GetVersion) (Variables|Default|GetColor)))