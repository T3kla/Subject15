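; BP_Emisor is a trigger volume that broadcasts when an actor tagged "Player" enters or leaves its box.
; Box overlap events update the inside and exit flags, then call the PlayerInside dispatcher with both values.
; Tick clears the exit flag whenever the player is outside, making it a short-lived pulse after leaving.
; The construction script sizes the box from an extent variable.
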(event OnComponentBeginOverlap(Box)
  (params (OverlappedComponent :type Primitive%20Component%20Object%20Reference) (OtherActor :type Actor%20Object%20Reference) (OtherComp :type Primitive%20Component%20Object%20Reference) (OtherBodyIndex :type Integer) (bFromSweep :type Boolean) (SweepResult :type Hit%20Result%20Structure%20%28by%20ref%29))
  (if (Actor|ActorHasTag OtherActor "Player")
    (Variables|Default|SetPlayerInside true)
    (Variables|Default|SetPlayterExit false)
    (Default|CallPlayerInsideDispatcher (Variables|Default|GetPlayerInside) (Variables|Default|GetPlayterExit))))

(event OnComponentEndOverlap(Box)
  (params (OverlappedComponent :type Primitive%20Component%20Object%20Reference) (OtherActor :type Actor%20Object%20Reference) (OtherComp :type Primitive%20Component%20Object%20Reference) (OtherBodyIndex :type Integer))
  (if (Actor|ActorHasTag OtherActor "Player")
    (Variables|Default|SetPlayerInside false)
    (Variables|Default|SetPlayterExit true)
    (Default|CallPlayerInsideDispatcher (Variables|Default|GetPlayerInside) (Variables|Default|GetPlayterExit))))

(event EventTick
  (params (DeltaSeconds :type Float%20%28single-precision%29))
  (if (not (Variables|Default|GetPlayerInside))
    (Variables|Default|SetPlayterExit false)))

(fn ConstructionScript
  (Components|Box|SetBoxExtent (Variables|Default|GetBox) (Variables|Default|GetIn%20Box%20Extent) true))